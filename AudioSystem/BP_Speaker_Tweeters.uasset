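; Configurable speaker prop with tweeters that plays music and visibly vibrates while it plays.
; The construction script shows the chosen speaker model and optional grate cover, sets the sound and volume, and can override materials.
; AutoPlay or Event_PlayMusic starts the audio and a timeline that randomly jitters both tweeter meshes, with SpeakerPower scaling shake and play rate.
; Event_StopMusic halts both, and both events are meant for Level Blueprint calls.
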(event `self.ReceiveBeginPlay`
  (bind _speakerpower (`self.SpeakerPower`))
  (bind _speakertweeter_tweeter1 (`self.SpeakerTweeter_Tweeter1`))
  (bind _speakertweeter_tweeter (`self.SpeakerTweeter_Tweeter`))
  (bind _returnvalue (`KismetMathLibrary.RandomFloatInRange` (* _speakerpower -0.05) (* _speakerpower 0.05)))
  (if (`self.AutoPlay?`)
    ;[1 1 1] If Music is playing then Vibrate Speaker System
    (`AudioComponent.Play` (`self.Audio`) 0.0 :!label _label)
    (`TimelineComponent.SetPlayRate` (`self.Timeline_0`) _speakerpower)
    (`Timeline|Timeline_0` :!label _label_2
      (:`Update`
        (`|ExecutionSequence`
          (:`then_0`
            (`/Engine/EditorBlueprintResources/StandardMacros.IsValid` _speakertweeter_tweeter
              (:`Is Valid`
                (`SceneComponent.K2_SetRelativeLocation` _speakertweeter_tweeter (`KismetMathLibrary.MakeVector` _returnvalue _returnvalue _returnvalue) false false))))
          (:`then_1`
            (`/Engine/EditorBlueprintResources/StandardMacros.IsValid` _speakertweeter_tweeter1
              (:`Is Valid`
                (`SceneComponent.K2_SetRelativeLocation` _speakertweeter_tweeter1 (`KismetMathLibrary.MakeVector` _returnvalue _returnvalue _returnvalue) false false)))))))))

(event `Event_PlayMusic`
  ;[1 1 1] Trigger on and off speaker system in game using level blueprint calling a reference with these events
  (goto _label))

(event `Event_StopMusic`
  ;[1 1 1] Trigger on and off speaker system in game using level blueprint calling a reference with these events
  ;[1 1 1] If Music is playing then Vibrate Speaker System
  (`AudioComponent.Stop` (`self.Audio`))
  (goto _label_2 :!via `Stop`))

(fn `UserConstructionScript`
  (bind _speakersleek_lp (`self.SpeakerSleek_LP`))
  (bind _audio (`self.Audio`))
  (`|ExecutionSequence`
    (:`then_0`
      ;[1 1 1] Set Basic Functionality
      (if (`self.Speaker1?`)
        (`SceneComponent.SetVisibility` _speakersleek_lp true false)
        (else
          (`SceneComponent.SetVisibility` _speakersleek_lp false false))))
    (:`then_1`
      (if (`self.Speaker2?`)
        (`SceneComponent.SetVisibility` (`self.SpeakerTweeter_Base`) true false)
        (`SceneComponent.SetVisibility` (`self.SpeakerTweeter_Frame2`) true false)
        (`SceneComponent.SetVisibility` (`self.SpeakerTweeter_Tweeter`) true false)
        (`SceneComponent.SetVisibility` (`self.SpeakerTweeter_Tweeter1`) true false)
        (`SceneComponent.SetVisibility` (`self.SpeakerBox_Multi_CablePanel`) true false)
        (`SceneComponent.SetVisibility` (`self.SpeakerTweeter_Frame1`) true false)
        (if (`self.Speaker2 Cover?`)
          (`SceneComponent.SetVisibility` (`self.GrateCover`) true false))))
    (:`then_2`
      (`/Engine/EditorBlueprintResources/StandardMacros.IsValid` _audio
        (:`Is Valid`
          (`AudioComponent.SetSound` _audio (`self.Select SoundMusic`))
          (`AudioComponent.SetVolumeMultiplier` (`self.Audio`) (`self.SoundMusic Volume`)))))
    (:`then_3`
      (if (`self.Set New Speaker Material?`)
        (`PrimitiveComponent.SetMaterial` (`self.SpeakerTweeter_Base`) 0 (`self.Select Speaker Material`))
        (`PrimitiveComponent.SetMaterial` (`self.SpeakerTweeter_Frame1`) 0 (`self.Select Speaker Material`))
        (`PrimitiveComponent.SetMaterial` (`self.SpeakerTweeter_Frame2`) 0 (`self.Select Speaker Material`))
        (`PrimitiveComponent.SetMaterial` (`self.SpeakerTweeter_Tweeter`) 0 (`self.Select Speaker Material`))
        (`PrimitiveComponent.SetMaterial` (`self.SpeakerBox_Multi_CablePanel`) 0 (`self.Select Speaker Material`))
        (`PrimitiveComponent.SetMaterial` (`self.SpeakerTweeter_Tweeter1`) 0 (`self.Select Speaker Material`))
        (`PrimitiveComponent.SetMaterial` (`self.SpeakerSleek_LP`) 0 (`self.Select Speaker Material`))))))