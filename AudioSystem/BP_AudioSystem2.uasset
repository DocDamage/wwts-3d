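; Configurable speaker system actor that plays music while vibrating up to four speaker cones.
; Construction script toggles the box and individual speakers with their collision, and applies sound, volume, box squash, materials and logo decals.
; AutoPlay or Event_PlayMusic starts the audio and a timeline, at a SpeakerPower play rate, that drives cone relative locations.
; Event_StopMusic halts both, and both events are meant to be called from the Level Blueprint.
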(event `self.ReceiveBeginPlay`
  (bind _cone2 (`self.Cone2`))
  (bind _cone3 (`self.Cone3`))
  (bind _cone4 (`self.Cone4`))
  (bind _cone (`self.Cone`))
  (if (`self.AutoPlay?`)
    ;[1 1 1] If Music is playing then Vibrate Speaker System
    (`AudioComponent.Play` (`self.Audio`) 0.0 :!label _label)
    (`TimelineComponent.SetPlayRate` (`self.Timeline_0`) (`self.SpeakerPower`))
    (bind (_direction _newtrack_0) (`Timeline|Timeline_0` :!label _label_2)
      (:`Update`
        (`|ExecutionSequence`
          (:`then_0`
            (`/Engine/EditorBlueprintResources/StandardMacros.IsValid` _cone
              (:`Is Valid`
                (`SceneComponent.K2_SetRelativeLocation` _cone _newtrack_0 false false))))
          (:`then_1`
            (`/Engine/EditorBlueprintResources/StandardMacros.IsValid` _cone2
              (:`Is Valid`
                (`SceneComponent.K2_SetRelativeLocation` _cone2 _newtrack_0 false false))))
          (:`then_2`
            (`/Engine/EditorBlueprintResources/StandardMacros.IsValid` _cone3
              (:`Is Valid`
                (`SceneComponent.K2_SetRelativeLocation` _cone3 _newtrack_0 false false))))
          (:`then_3`
            (`/Engine/EditorBlueprintResources/StandardMacros.IsValid` _cone4
              (:`Is Valid`
                (`SceneComponent.K2_SetRelativeLocation` _cone4 _newtrack_0 false false)))))))))

(event `Event_PlayMusic`
  ;[1 1 1] Trigger on and off speaker system in game using level blueprint calling a reference with these events
  (goto _label))

(event `Event_StopMusic`
  ;[1 1 1] Trigger on and off speaker system in game using level blueprint calling a reference with these events
  ;[1 1 1] If Music is playing then Vibrate Speaker System
  (`AudioComponent.Stop` (`self.Audio`))
  (goto _label_2 :!via `Stop`))

(fn `UserConstructionScript`
  (bind _set_decals_logos_ (`self.Set Decals Logos?`))
  (bind _framenmagnet (`self.FrameNMagnet`))
  (bind _framenmagnet4 (`self.FrameNMagnet4`))
  (bind _audio (`self.Audio`))
  (bind _speaker2_ (`self.Speaker2?`))
  (bind _framenmagnet2 (`self.FrameNMagnet2`))
  (bind _speaker3_ (`self.Speaker3?`))
  (bind _framenmagnet3 (`self.FrameNMagnet3`))
  (bind _speaker1_ (`self.Speaker1?`))
  (bind _speaker4_ (`self.Speaker4?`))
  ;[1 1 1] Set Basics
  (`|ExecutionSequence`
    (:`then_0`
      (if (`self.SpeakerBox?`)
        (`|ExecutionSequence`
          (:`then_0`
            ;[1 1 1] If SpeakerBox is used, select speakers to be used in the box
            (`PrimitiveComponent.SetCollisionEnabled` (`self.SpeakerBox`) "QueryAndPhysics"))
          (:`then_1`
            (`SceneComponent.SetVisibility` (`self.FrameNMagnet`) _speaker1_ false)
            (`SceneComponent.SetVisibility` (`self.Connectors`) _speaker1_ false)
            (`SceneComponent.SetVisibility` (`self.Spider`) _speaker1_ false)
            (`SceneComponent.SetVisibility` (`self.Cone`) _speaker1_ false)
            (`SceneComponent.SetVisibility` (`self.VoiceCoil`) _speaker1_ false)
            (`SceneComponent.SetVisibility` (`self.Speaker1SelectionIcon`) _speaker1_ false)
            (if _speaker1_
              (`PrimitiveComponent.SetCollisionEnabled` _framenmagnet "QueryAndPhysics")
              (if _set_decals_logos_
                (`SceneComponent.SetVisibility` (`self.Decal`) true false))
              (else
                (`PrimitiveComponent.SetCollisionEnabled` _framenmagnet "NoCollision"))))
          (:`then_2`
            (`SceneComponent.SetVisibility` (`self.FrameNMagnet2`) _speaker2_ false)
            (`SceneComponent.SetVisibility` (`self.Connectors2`) _speaker2_ false)
            (`SceneComponent.SetVisibility` (`self.Cone2`) _speaker2_ false)
            (`SceneComponent.SetVisibility` (`self.VoiceCoil2`) _speaker2_ false)
            (`SceneComponent.SetVisibility` (`self.Spider2`) _speaker2_ false)
            (`SceneComponent.SetVisibility` (`self.Speaker2SelectionIcon`) _speaker2_ false)
            (if _speaker2_
              (`PrimitiveComponent.SetCollisionEnabled` _framenmagnet2 "QueryAndPhysics")
              (if _set_decals_logos_
                (`SceneComponent.SetVisibility` (`self.Decal2`) true false))
              (else
                (`PrimitiveComponent.SetCollisionEnabled` _framenmagnet2 "NoCollision"))))
          (:`then_3`
            (`SceneComponent.SetVisibility` (`self.FrameNMagnet3`) _speaker3_ false)
            (`SceneComponent.SetVisibility` (`self.Connectors3`) _speaker3_ false)
            (`SceneComponent.SetVisibility` (`self.Cone3`) _speaker3_ false)
            (`SceneComponent.SetVisibility` (`self.VoiceCoil3`) _speaker3_ false)
            (`SceneComponent.SetVisibility` (`self.Spider3`) _speaker3_ false)
            (`SceneComponent.SetVisibility` (`self.Speaker3Selection`) _speaker3_ false)
            (if _speaker3_
              (`PrimitiveComponent.SetCollisionEnabled` _framenmagnet3 "QueryAndPhysics")
              (if _set_decals_logos_
                (`SceneComponent.SetVisibility` (`self.Decal3`) true false))
              (else
                (`PrimitiveComponent.SetCollisionEnabled` _framenmagnet3 "NoCollision"))))
          (:`then_4`
            (`SceneComponent.SetVisibility` (`self.FrameNMagnet4`) _speaker4_ false)
            (`SceneComponent.SetVisibility` (`self.Connectors4`) _speaker4_ false)
            (`SceneComponent.SetVisibility` (`self.Cone4`) _speaker4_ false)
            (`SceneComponent.SetVisibility` (`self.VoiceCoil4`) _speaker4_ false)
            (`SceneComponent.SetVisibility` (`self.Spider4`) _speaker4_ false)
            (`SceneComponent.SetVisibility` (`self.Speaker4Selection`) _speaker4_ false)
            (if _speaker4_
              (`PrimitiveComponent.SetCollisionEnabled` _framenmagnet4 "QueryAndPhysics")
              (if _set_decals_logos_
                (`SceneComponent.SetVisibility` (`self.Decal4`) true false))
              (else
                (`PrimitiveComponent.SetCollisionEnabled` _framenmagnet4 "NoCollision")))))
        (else
          ;[1 1 1] If SpeakerBox is not used, then remove a speaker and set the other's location to the center of the BP
          (`|ExecutionSequence`
            (:`then_0`
              (`SceneComponent.SetVisibility` (`self.FrameNMagnet`) true false)
              (`SceneComponent.SetVisibility` (`self.Connectors`) true false)
              (`SceneComponent.SetVisibility` (`self.Spider`) true false)
              (`SceneComponent.SetVisibility` (`self.Cone`) true false)
              (`SceneComponent.SetVisibility` (`self.VoiceCoil`) true false)
              (`SceneComponent.SetVisibility` (`self.Speaker1SelectionIcon`) true false)
              (`SceneComponent.SetVisibility` (`self.FrameNMagnet2`) false false)
              (`SceneComponent.SetVisibility` (`self.Connectors2`) false false)
              (`SceneComponent.SetVisibility` (`self.Cone2`) false false)
              (`SceneComponent.SetVisibility` (`self.VoiceCoil2`) false false)
              (`SceneComponent.SetVisibility` (`self.Spider2`) false false)
              (`SceneComponent.SetVisibility` (`self.Speaker2SelectionIcon`) false false))
            (:`then_1`
              (`SceneComponent.K2_SetRelativeLocation` (`self.Speaker1SelectionIcon`) (0.0 0.0 0.0) false false)
              (`PrimitiveComponent.SetCollisionEnabled` (`self.SpeakerBox`) "NoCollision")
              (`PrimitiveComponent.SetCollisionEnabled` (`self.FrameNMagnet2`) "NoCollision"))))))
    (:`then_1`
      (`SceneComponent.SetVisibility` (`self.SpeakerBox`) (`self.SpeakerBox?`) false))
    (:`then_2`
      (`AudioComponent.SetSound` _audio (`self.Select SoundMusic`))
      (`AudioComponent.SetVolumeMultiplier` _audio (`self.SoundMusic Volume`)))
    (:`then_3`
      (if (`self.ShrinkBox`)
        (`self.SetActorScale3D` (1.0 1.0 0.85))
        (else
          (`self.SetActorScale3D` (1.0 1.0 1.0)))))
    (:`then_4`
      (if (`self.SpeakerBox New Material?`)
        (`PrimitiveComponent.SetMaterial` (`self.SpeakerBox`) 0 (`self.SpeakerBox Material`))))
    (:`then_5`
      (if (`self.Speaker New Material?`)
        (`PrimitiveComponent.SetMaterial` (`self.Cone`) 0 (`self.Speaker Material?`))
        (`PrimitiveComponent.SetMaterial` (`self.Cone2`) 0 (`self.Speaker Material?`))
        (`PrimitiveComponent.SetMaterial` (`self.Cone3`) 0 (`self.Speaker Material?`))
        (`PrimitiveComponent.SetMaterial` (`self.Cone4`) 0 (`self.Speaker Material?`))))
    (:`then_6`
      (if (`self.Set Decals Logos?`)
        (`DecalComponent.SetDecalMaterial` (`self.Decal2`) (`self.Select Decal Logos`))
        (`DecalComponent.SetDecalMaterial` (`self.Decal`) (`self.Select Decal Logos`))
        (`DecalComponent.SetDecalMaterial` (`self.Decal4`) (`self.Select Decal Logos`))
        (`DecalComponent.SetDecalMaterial` (`self.Decal3`) (`self.Select Decal Logos`))))))