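; Configurable speaker prop that plays a selected sound and animates its cones to look like they vibrate.
; Construction script sets the sound, volume, materials and logo decals, and toggles visibility and collision for dual-box, single-box or unboxed speaker layouts.
; Playback starts with AutoPlay or Event_PlayMusic, while a timeline at SpeakerPower rate moves both cones.
; Event_StopMusic halts audio and timeline; motion does not analyze the audio.
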(event `self.ReceiveBeginPlay`
  (bind _cone2 (`self.Cone2`))
  (bind _cone (`self.Cone`))
  (if (`self.AutoPlay?`)
    ;[1 1 1] If Music is playing then Vibrate Speaker System
    (`AudioComponent.Play` (`self.Audio`) 0.0 :!label _label)
    (`TimelineComponent.SetPlayRate` (`self.Timeline_0`) (`self.SpeakerPower`))
    (bind (_direction _newtrack_0) (`Timeline|Timeline_0` :!label _label_2)
      (:`Update`
        (`|ExecutionSequence`
          (:`then_0`
            (`/Engine/EditorBlueprintResources/StandardMacros.IsValid` _cone
              (:`Is Valid`
                (`SceneComponent.K2_SetRelativeLocation` _cone _newtrack_0 false false))))
          (:`then_1`
            (`/Engine/EditorBlueprintResources/StandardMacros.IsValid` _cone2
              (:`Is Valid`
                (`SceneComponent.K2_SetRelativeLocation` _cone2 _newtrack_0 false false)))))))))

(event `Event_PlayMusic`
  ;[1 1 1] Trigger on and off speaker system in game using level blueprint calling a reference with these events
  (goto _label))

(event `Event_StopMusic`
  ;[1 1 1] Trigger on and off speaker system in game using level blueprint calling a reference with these events
  ;[1 1 1] If Music is playing then Vibrate Speaker System
  (`AudioComponent.Stop` (`self.Audio`))
  (goto _label_2 :!via `Stop`))

(fn `UserConstructionScript`
  (bind _framenmagnet (`self.FrameNMagnet`))
  (bind _framenmagnet2 (`self.FrameNMagnet2`))
  (bind _speaker1_ (`self.Speaker1?`))
  (bind _speaker2_ (`self.Speaker2?`))
  (`|ExecutionSequence`
    (:`then_0`
      ;[1 1 1] Set SpeakerBox + SoundMusic file
      (`SceneComponent.SetVisibility` (`self.SpeakerBox`) (`self.DualSpeakerBox?`) false)
      (`AudioComponent.SetSound` (`self.Audio`) (`self.Select SoundMusic`))
      (if (`self.DualSpeakerBox?`)
        ;[1 1 1] If SpeakerBox is used, select either speaker or both to be used in the box
        (`|ExecutionSequence`
          (:`then_0`
            (`PrimitiveComponent.SetCollisionEnabled` (`self.SpeakerBox`) "QueryAndPhysics")
            (`PrimitiveComponent.SetCollisionEnabled` (`self.SpeakerBox_Single`) "NoCollision")
            (`PrimitiveComponent.SetCollisionEnabled` (`self.CablePanel`) "NoCollision"))
          (:`then_1`
            (`SceneComponent.SetVisibility` (`self.FrameNMagnet`) _speaker1_ false)
            (`SceneComponent.SetVisibility` (`self.Connectors`) _speaker1_ false)
            (`SceneComponent.SetVisibility` (`self.Spider`) _speaker1_ false)
            (`SceneComponent.SetVisibility` (`self.Cone`) _speaker1_ false)
            (`SceneComponent.SetVisibility` (`self.VoiceCoil`) _speaker1_ false)
            (`SceneComponent.SetVisibility` (`self.Speaker1SelectionIcon`) _speaker1_ false)
            (if _speaker1_
              (`PrimitiveComponent.SetCollisionEnabled` _framenmagnet "QueryAndPhysics")
              (else
                (`PrimitiveComponent.SetCollisionEnabled` _framenmagnet "NoCollision"))))
          (:`then_2`
            (`SceneComponent.SetVisibility` (`self.FrameNMagnet2`) _speaker2_ false)
            (`SceneComponent.SetVisibility` (`self.Connectors2`) _speaker2_ false)
            (`SceneComponent.SetVisibility` (`self.Cone2`) _speaker2_ false)
            (`SceneComponent.SetVisibility` (`self.VoiceCoil2`) _speaker2_ false)
            (`SceneComponent.SetVisibility` (`self.Spider2`) _speaker2_ false)
            (`SceneComponent.SetVisibility` (`self.Speaker2SelectionIcon`) _speaker2_ false)
            (if _speaker2_
              (`PrimitiveComponent.SetCollisionEnabled` _framenmagnet2 "QueryAndPhysics")
              (else
                (`PrimitiveComponent.SetCollisionEnabled` _framenmagnet2 "NoCollision"))))
          (:`then_3`
            (if (`self.Set Decals Logos?`)
              (`SceneComponent.SetVisibility` (`self.Decal`) true false)
              (`SceneComponent.SetVisibility` (`self.Decal2`) true false))))
        (else
          ;[1 1 1] If SpeakerBox is not used, then remove a speaker and set the other's location to the center of the BP
          (`|ExecutionSequence`
            (:`then_0`
              (`SceneComponent.SetVisibility` (`self.FrameNMagnet`) true false)
              (`SceneComponent.SetVisibility` (`self.Connectors`) true false)
              (`SceneComponent.SetVisibility` (`self.Spider`) true false)
              (`SceneComponent.SetVisibility` (`self.Cone`) true false)
              (`SceneComponent.SetVisibility` (`self.VoiceCoil`) true false)
              (`SceneComponent.SetVisibility` (`self.Speaker1SelectionIcon`) true false)
              (`SceneComponent.SetVisibility` (`self.FrameNMagnet2`) false false)
              (`SceneComponent.SetVisibility` (`self.Connectors2`) false false)
              (`SceneComponent.SetVisibility` (`self.Cone2`) false false)
              (`SceneComponent.SetVisibility` (`self.VoiceCoil2`) false false)
              (`SceneComponent.SetVisibility` (`self.Spider2`) false false)
              (`SceneComponent.SetVisibility` (`self.Speaker2SelectionIcon`) false false)
              (`SceneComponent.SetVisibility` (`self.Decal2`) false false)
              (`SceneComponent.SetVisibility` (`self.Decal`) (`self.Set Decals Logos?`) false))
            (:`then_1`
              (`SceneComponent.K2_SetRelativeLocation` (`self.Speaker1SelectionIcon`) (0.0 0.0 0.0) false false)
              (`PrimitiveComponent.SetCollisionEnabled` (`self.SpeakerBox`) "NoCollision")
              (`PrimitiveComponent.SetCollisionEnabled` (`self.FrameNMagnet2`) "NoCollision")
              (`PrimitiveComponent.SetCollisionEnabled` (`self.SpeakerBox_Single`) "NoCollision")
              (`PrimitiveComponent.SetCollisionEnabled` (`self.CablePanel`) "NoCollision"))
            (:`then_2`
              (if (`self.SingleSpeakerBox?`)
                (`SceneComponent.SetVisibility` (`self.SpeakerBox_Single`) true false)
                (`SceneComponent.SetVisibility` (`self.CablePanel`) true false)
                (`PrimitiveComponent.SetCollisionEnabled` (`self.CablePanel`) "QueryAndPhysics")
                (`PrimitiveComponent.SetCollisionEnabled` (`self.SpeakerBox_Single`) "QueryAndPhysics")))))))
    (:`then_1`
      (`AudioComponent.SetVolumeMultiplier` (`self.Audio`) (`self.SoundMusic Volume`)))
    (:`then_2`
      (if (`self.SpeakerBox New Material?`)
        (`PrimitiveComponent.SetMaterial` (`self.SpeakerBox`) 0 (`self.SpeakerBox Material`))
        (`PrimitiveComponent.SetMaterial` (`self.SpeakerBox_Single`) 0 (`self.SpeakerBox Material`))))
    (:`then_3`
      (if (`self.Speaker New Material?`)
        (`PrimitiveComponent.SetMaterial` (`self.Cone`) 0 (`self.Speaker Material?`))
        (`PrimitiveComponent.SetMaterial` (`self.Cone2`) 0 (`self.Speaker Material?`))))
    (:`then_4`
      (if (`self.Set Decals Logos?`)
        (`DecalComponent.SetDecalMaterial` (`self.Decal2`) (`self.Select Decal Logos`))
        (`DecalComponent.SetDecalMaterial` (`self.Decal`) (`self.Select Decal Logos`))))))